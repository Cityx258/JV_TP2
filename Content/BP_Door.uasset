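; BP_Door is an interactable hinged door that swings open and closed by rotating its Pivot 90 degrees in yaw.
; A single timeline lerps the rotation, playing forward to open and reversing to close, and sets DoorState when it finishes.
; Interact calls Toggle, which picks Open or Close from DoorState, so interacting mid-swing reverses the door's motion.
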(event Custom|Open%20Door
  (Variables|Default|SetDoor%20State "NewEnumerator2")
  (bind (_direction _alpha) (Timeline|Timeline Play)
    (:Update
      (Transformation|SetRelativeRotation (Variables|Default|GetPivot) (Math|Rotator|MakeRotator 0.0 0.0 (Math|Float|Lerp 0.0 -9e+01 _alpha)) false false))
    (:Finished
      (switch Utilities|FlowControl|Switch|SwitchonETimelineDirection _direction
        (:Forward
          (Variables|Default|SetDoor%20State "NewEnumerator0"))
        (:Backward
          (Variables|Default|SetDoor%20State "NewEnumerator1"))))))

(event Custom|Close%20Door
  (Variables|Default|SetDoor%20State "NewEnumerator3")
  (bind (_direction _alpha) (Timeline|Timeline Reverse)
    (:Update
      (Transformation|SetRelativeRotation (Variables|Default|GetPivot) (Math|Rotator|MakeRotator 0.0 0.0 (Math|Float|Lerp 0.0 -9e+01 _alpha)) false false))
    (:Finished
      (switch Utilities|FlowControl|Switch|SwitchonETimelineDirection _direction
        (:Forward
          (Variables|Default|SetDoor%20State "NewEnumerator0"))
        (:Backward
          (Variables|Default|SetDoor%20State "NewEnumerator1"))))))

(event EventBeginPlay)

(event EventTick
  (params (DeltaSeconds :type Float%20%28single-precision%29)))

(event EventInteract
  (CallFunction|Toggle))

(fn ConstructionScript)

(fn Open
  (CallFunction|OpenDoor))

(fn Close
  (CallFunction|CloseDoor))

(fn Toggle
  (switch Utilities|FlowControl|Switch|SwitchonE_DoorState (Variables|Default|GetDoor%20State)
    (:NewEnumerator0
      (CallFunction|Close :!label _label))
    (:NewEnumerator1
      (CallFunction|Open :!label _label_2))
    (:NewEnumerator2
      (goto _label))
    (:NewEnumerator3
      (goto _label_2))))