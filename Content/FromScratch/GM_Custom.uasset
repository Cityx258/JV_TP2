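; GM_Custom is a game mode that checks the victory condition for collecting coins and chests.
; On BeginPlay it binds to the coin and chest collection events on the first player's PS_Custom player state.
; Each event stores the new count and runs CheckVictory, which pauses the game only when both totals reach their required amounts.
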(event Custom|Coin%20Collected
  (params (coins%20collected :type Integer))
  (bind _output_get (Variables|Default|SetCoins%20collected coins%20collected))
  (CallFunction|CheckVictory _output_get (Variables|Default|GetChests%20collected)))

(event Custom|Chest%20Collected
  (params (chests%20collected :type Integer))
  (bind _output_get (Variables|Default|SetChests%20collected chests%20collected))
  (CallFunction|CheckVictory (Variables|Default|GetCoins%20collected) _output_get))

(event EventBeginPlay
  (bind _asps_custom (Utilities|Casting|CastToPS_Custom (Game|GetPlayerState 0)))
  (EventDispatchers|BindEventtoOnCoinCollected _asps_custom (delegate Custom|Coin%20Collected))
  (EventDispatchers|BindEventtoOnChestCollected _asps_custom (delegate Custom|Chest%20Collected)))

(fn ConstructionScript)

(fn CheckVictory
  (params (Coins%20Collected :type Integer) (Chest%20Collected :type Integer))
  (Game|SetGamePaused (and (>= Coins%20Collected (Variables|Default|GetCoins%20Required)) (>= Chest%20Collected (Variables|Default|Getchests%20Required)))))